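; Player pawn for a rolling physics character, driven by torque on its static mesh from the forward and sideways axes.
; BeginPlay starts a camera fade and adds the HUD.
; Any damage triggers a one-time fade, whose returned duration times the delay before reloading the current level.
; The quit button flip-flops the pause menu, game pause, input mode and cursor, while AdjustSpringArm sets camera distance and pitch.
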(event EventBeginPlay
  ;[1 1 1] Camera Fade at begining of gameplay
  (CameraFades|StartCameraFade :self (Game|GetPlayerCameraManager 0) :Duration 3.0)
  ;[1 1 1] Adding HUD to viewport
  (bind _returnvalue (UserInterface|CreateWidget "/Game/UI/HUD/WBP_HUD.WBP_HUD_C"))
  (UserInterface|Viewport|AddtoViewport _returnvalue 0))

(event Game|Damage|EventAnyDamage
  (params (Damage :type Float%20%28single-precision%29) (DamageType :type Damage%20Type%20Object%20Reference) (InstigatedBy :type Controller%20Object%20Reference) (DamageCauser :type Actor%20Object%20Reference))
  ;[1 1 1] HandlingDeath
  (Utilities|FlowControl|DoOnce false
    (:Completed
      (bind _returnvalue (CallFunction|CameraFade))
      (Utilities|FlowControl|Delay _returnvalue)
      (CallFunction|RestartLevel))))

(event Input|ActionEvents|InputActionQuitButton
  (params (Key :type Key%20Structure :default "None"))
  (bind _returnvalue (Game|GetPlayerController 0))
  (bind _returnvalue_2 (Game|GetPlayerController 0))
  (:Pressed
    (Utilities|FlowControl|FlipFlop
      (:A
        (bind _returnvalue_3 (UserInterface|CreateWidget "/Game/UI/PauseMenu/WBP_PauseMenu.WBP_PauseMenu_C"))
        (UserInterface|Viewport|AddtoViewport _returnvalue_3 0)
        (Game|SetGamePaused true)
        (Input|SetInputModeUIOnly _returnvalue_2 0 "DoNotLock")
        (Variables|/Script/Engine.PlayerController|SetbShowMouseCursor _returnvalue_2 true))
      (:B
        (Widget|RemovefromParent _returnvalue_3)
        (Input|SetInputModeGameOnly _returnvalue)
        (Variables|/Script/Engine.PlayerController|SetbShowMouseCursor _returnvalue false)
        (Game|SetGamePaused false)))))

(event Input|AxisEvents|InputAxisMoveForward
  (params (AxisValue :type Float%20%28single-precision%29))
  ;[1 1 1] MovementForward
  (Class|PrimitiveComponent|AddTorqueinRadians (Variables|Default|GetStaticMesh) (Math|Vector|MakeVector 0.0 (* AxisValue (Variables|Default|GetRollSpeed)) 0.0) "None" true))

(event Input|AxisEvents|InputAxisMoveRight
  (params (AxisValue :type Float%20%28single-precision%29))
  ;[1 1 1] MovementSides
  (Class|PrimitiveComponent|AddTorqueinRadians (Variables|Default|GetStaticMesh) (Math|Vector|MakeVector (* AxisValue (* -1 (Variables|Default|GetRollSpeed))) 0.0 0.0) "None" true))

(fn ConstructionScript)

(fn CameraFade
  (bind _returnvalue (Math|Float|MakeLiteralFloat 2.0))
  (CameraFades|StartCameraFade :self (Game|GetPlayerCameraManager 0) :ToAlpha 1.0 :Duration _returnvalue)
  (return _returnvalue))

(fn RestartLevel
  (bind _returnvalue (Game|GetCurrentLevelName true))
  (Game|OpenLevel(byName) (Utilities|String|StringToName _returnvalue)))

(fn AdjustSpringArm
  (params (Distance :type Float%20%28double-precision%29) (Pitch :type Float%20%28double-precision%29))
  (bind _springarm (Variables|Default|GetSpringArm))
  (Variables|/Script/Engine.SpringArmComponent|SetTargetArmLength _springarm Distance)
  (Transformation|SetWorldRotation _springarm (Math|Rotator|MakeRotator 0.0 Pitch 0.0) false false))